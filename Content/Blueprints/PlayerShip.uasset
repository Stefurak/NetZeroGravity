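; Player ship actor that trails a spawned CursorNear actor and fires lasers on input.
; Each tick it interpolates toward a point offset along the cursor's forward axis by FollowDistance and rotates to face the cursor.
; Holding Fire opens a gate that spawns LaserProjectiles from LaserSpawn aimed at the Sphere component, re-entering through a retriggerable delay for auto-fire until release closes it.
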(event `self.ReceiveBeginPlay`
  (bind _followtargetactor (`self.FollowTargetActor`))
  ;[1 1 1] Spawns Cursor Near and sets Location to target
  (`self.EnableInput` (`GameplayStatics.GetPlayerController` 0))
  (bind _returnvalue (`|SpawnActorFromClass` "/Game/Blueprints/CursorNear.CursorNear_C" (`KismetMathLibrary.MakeTransform` (`self.K2_GetActorLocation`)) "Undefined" "OverrideRootScale"))
  (set `self.FollowTargetActor` _returnvalue)
  (`self.K2_SetActorLocationAndRotation` (`self.K2_GetActorLocation` _followtargetactor) (`self.K2_GetActorRotation` _followtargetactor)))

(event `self.ReceiveTick`
  (params (DeltaSeconds :type "Float (single-precision)"))
  (bind _returnvalue (`GameplayStatics.GetWorldDeltaSeconds`))
  (bind _followtargetactor (`self.FollowTargetActor`))
  ;[1 1 1] Ship Following Target (Cursor Near)
  (`self.K2_SetActorLocationAndRotation` (`KismetMathLibrary.VInterpTo` (`self.K2_GetActorLocation`) (+ (`self.K2_GetActorLocation` _followtargetactor) (* (`KismetMathLibrary.GetForwardVector` (`self.K2_GetActorRotation` _followtargetactor)) (`self.followDistance`))) _returnvalue (`self.followSpeed`)) (`KismetMathLibrary.RInterpTo` (`self.K2_GetActorRotation`) (`KismetMathLibrary.FindLookAtRotation` (`self.K2_GetActorLocation`) (`self.K2_GetActorLocation` _followtargetactor)) _returnvalue 50.0)))

(event `InputAction|InputAction Fire`
  (params (Key :type "Key Structure" :default "AnyKey"))
  (bind _returnvalue (`SceneComponent.K2_GetComponentLocation` (`self.LaserSpawn`)))
  (:`Pressed`
    (`|ExecutionSequence`
      (:`then_0`
        (goto _label :!via `Open`))
      (:`then_1`
        (`/Engine/EditorBlueprintResources/StandardMacros.Gate` true :!label _label
          (:`Exit`
            (`|ExecutionSequence`
              (:`then_0`
                (`|SpawnActorFromClass` "/Game/Blueprints/LaserProjectile.LaserProjectile_C" (`KismetMathLibrary.MakeTransform` _returnvalue (`KismetMathLibrary.FindLookAtRotation` _returnvalue (`SceneComponent.K2_GetComponentLocation` (`self.Sphere`)))) "Undefined" "OverrideRootScale"))
              (:`then_1`
                (`KismetSystemLibrary.RetriggerableDelay` 0.5)
                (goto _label))))))))
  (:`Released`
    (goto _label :!via `Close`)))

(fn `UserConstructionScript`)