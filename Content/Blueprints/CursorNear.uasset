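; CursorNear is an actor that trails a point a set distance in front of the first player's pawn, apparently as a near cursor.
; BeginPlay caches the pawn and makes a first move.
; Each Tick, it projects FollowDistance along the pawn's forward vector and eases toward that point with VInterpTo at FollowSpeed.
; The combined location-and-rotation setter receives only a location, so rotation does not track the pawn.
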(event `self.ReceiveBeginPlay`
  (bind _playerpawn (`self.PlayerPawn`))
  (set `self.PlayerPawn` (`GameplayStatics.GetPlayerPawn` 0))
  (`self.K2_SetActorLocationAndRotation` (`KismetMathLibrary.VInterpTo` (`self.K2_GetActorLocation`) (+ (`self.K2_GetActorLocation` _playerpawn) (* (`KismetMathLibrary.GetForwardVector` (`self.K2_GetActorRotation` _playerpawn)) (`self.followDistance`))) (`GameplayStatics.GetWorldDeltaSeconds`) (`self.followSpeed`)) (struct)))

(event `self.ReceiveTick`
  (params (DeltaSeconds :type "Float (single-precision)"))
  (bind _playerpawn (`self.PlayerPawn`))
  (`self.K2_SetActorLocationAndRotation` (`KismetMathLibrary.VInterpTo` (`self.K2_GetActorLocation`) (+ (`self.K2_GetActorLocation` _playerpawn) (* (`KismetMathLibrary.GetForwardVector` (`self.K2_GetActorRotation` _playerpawn)) (`self.followDistance`))) (`GameplayStatics.GetWorldDeltaSeconds`) (`self.followSpeed`))))

(fn `UserConstructionScript`)