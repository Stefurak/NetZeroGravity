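; EnemyShip is an enemy actor that flies along its root's forward vector each Tick, without sweeping, until player bullets destroy it.
; Overlapping an actor tagged PlayerBullet destroys that actor and decrements EnemyHealth.
; Tick switches on EnemyHealth to hide health indicator components as it drops and destroys the ship at zero.
; Yaw-only logic to turn the health pivot toward a camera is present but unconnected.
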(event `self.ReceiveBeginPlay`)

(event `self.ReceiveTick`
  (params (DeltaSeconds :type "Float (single-precision)"))
  (`self.K2_SetActorLocation` (+ (* (`SceneComponent.GetForwardVector` (`self.DefaultSceneRoot`)) (`self.travelSpeed`)) (`self.K2_GetActorLocation`)))
  ;[1 1 1] HealthBars on Top When Hit
  (switch `int` (`self.enemyHealth`)
    (:`0`
      (`self.K2_DestroyActor`))
    (:`1`
      (`SceneComponent.SetVisibility` (`self.health2`) false false))
    (:`2`
      (`SceneComponent.SetVisibility` (`self.health3`) false false))))

(event `self.ReceiveActorBeginOverlap`
  (params (OtherActor :type "Actor Object Reference"))
  (if (`self.ActorHasTag` OtherActor "PlayerBullet")
    (`self.K2_DestroyActor` OtherActor)
    (`/Engine/EditorBlueprintResources/StandardMacros.DecrementInt` (`self.enemyHealth`))))

(fn `UserConstructionScript`)