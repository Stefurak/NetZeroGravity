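; GameCam_BP is a follow camera that spawns the PlayerShip at its own location on BeginPlay and serves as the player's view target.
; Each Tick it reasserts itself as view target with zero blend and interpolates toward a point offset along the ship's up and forward axes.
; VInterpTo and RInterpTo smooth position and rotation, both driven by FollowSpeed, with FollowDistance setting the forward offset.
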(event `self.ReceiveBeginPlay`
  (bind _returnvalue (`GameplayStatics.GetWorldDeltaSeconds`))
  (bind _followspeed (`self.followSpeed`))
  (bind _followtargetactor (`self.FollowTargetActor`))
  (bind _returnvalue_2 (`self.K2_GetActorRotation` _followtargetactor))
  (bind _returnvalue_3 (`|SpawnActorFromClass` "/Game/Blueprints/PlayerShip.PlayerShip_C" (`KismetMathLibrary.MakeTransform` (`self.K2_GetActorLocation`)) "Undefined" "OverrideRootScale"))
  (set `self.FollowTargetActor` _returnvalue_3)
  (bind _output_get (set `self.PlayerPawn` (`GameplayStatics.GetPlayerPawn` 0)))
  (bind _asplayer_controller (cast `PlayerController` (`Pawn.GetController` _output_get)))
  (`PlayerController.SetViewTargetWithBlend` _asplayer_controller self 0.0 "VTBlend_Linear" 0.0 false)
  (`self.K2_SetActorLocationAndRotation` (`KismetMathLibrary.VInterpTo` (`self.K2_GetActorLocation`) (+ (`self.K2_GetActorLocation` _followtargetactor) (* (`KismetMathLibrary.GetUpVector` _returnvalue_2) 50.0) (* (`KismetMathLibrary.GetForwardVector` _returnvalue_2) (`self.followDistance`))) _returnvalue _followspeed) (`KismetMathLibrary.RInterpTo` (`self.K2_GetActorRotation`) _returnvalue_2 _returnvalue _followspeed)))

(event `self.ReceiveTick`
  (params (DeltaSeconds :type "Float (single-precision)"))
  (bind _returnvalue (`GameplayStatics.GetWorldDeltaSeconds`))
  (bind _followspeed (`self.followSpeed`))
  (bind _followtargetactor (`self.FollowTargetActor`))
  (bind _returnvalue_2 (`self.K2_GetActorRotation` _followtargetactor))
  (`PlayerController.SetViewTargetWithBlend` (stale `self.ReceiveBeginPlay` _asplayer_controller) self 0.0 "VTBlend_Linear" 0.0 false)
  (`self.K2_SetActorLocationAndRotation` (`KismetMathLibrary.VInterpTo` (`self.K2_GetActorLocation`) (+ (`self.K2_GetActorLocation` _followtargetactor) (* (`KismetMathLibrary.GetUpVector` _returnvalue_2) 50.0) (* (`KismetMathLibrary.GetForwardVector` _returnvalue_2) (`self.followDistance`))) _returnvalue _followspeed) (`KismetMathLibrary.RInterpTo` (`self.K2_GetActorRotation`) _returnvalue_2 _returnvalue _followspeed)))

(fn `UserConstructionScript`)