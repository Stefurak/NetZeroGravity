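; Player Blueprint that keeps the actor inside a bounded corridor and ends the run at a fixed distance along X.
; Each tick, once X passes a hardcoded threshold it opens MainMenuLevel.
; Otherwise it clamps Y between MaxLeft and MaxRight and Z between MaxDown and MaxUp, setting the location directly without sweep.
; BeginPlay and the construction script are empty.
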(event `self.ReceiveBeginPlay`)

(event `self.ReceiveTick`
  (params (DeltaSeconds :type "Float (single-precision)"))
  (if (> (.x (`self.K2_GetActorLocation`)) 36000.0)
    (`GameplayStatics.OpenLevel` "MainMenuLevel")
    (else
      (`self.K2_SetActorLocation` (`KismetMathLibrary.MakeVector` (.x (`self.K2_GetActorLocation`)) (`KismetMathLibrary.FClamp` (.y (`self.K2_GetActorLocation`)) (`self.maxLeft`) (`self.maxRight`)) (`KismetMathLibrary.FClamp` (.z (`self.K2_GetActorLocation`)) (`self.maxDown`) (`self.maxUp`)))))))

(fn `UserConstructionScript`)